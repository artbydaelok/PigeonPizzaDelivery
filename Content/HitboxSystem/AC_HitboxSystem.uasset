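; AC_HitboxSystem is an actor component that turns its owner's box component into a damaging hitbox against the player.
; On BeginPlay it caches the BP_ThirdPersonCharacter found in the level and binds to the begin-overlap event of the owner's BoxComponent.
; When the overlapping actor is that player, it applies a fixed amount of damage.
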(event Custom|HitSomething
  (params (OverlappedComponent :type Primitive%20Component%20Object%20Reference) (OtherActor :type Actor%20Object%20Reference) (OtherComp :type Primitive%20Component%20Object%20Reference) (OtherBodyIndex :type Integer) (bFromSweep :type Boolean) (SweepResult :type Hit%20Result%20Structure%20%28by%20ref%29))
  (if (== OtherActor (Variables|Default|GetPlayer))
    (Default|TakeDamage (Variables|Default|GetPlayer) 5.0)))

(event EventBeginPlay
  (bind _returnvalue (Actor|GetActorOfClass "/Game/ThirdPerson/Blueprints/BP_ThirdPersonCharacter.BP_ThirdPersonCharacter_C"))
  (Variables|Default|SetPlayer _returnvalue)
  (Variables|Default|SetHitboxArea (Actor|GetComponentbyClass (Components|GetOwner) "/Script/Engine.BoxComponent"))
  (Collision|BindEventtoOnComponentBeginOverlap (Variables|Default|GetHitboxArea) (delegate Custom|HitSomething)))

(event EventTick
  (params (DeltaSeconds :type Float%20%28single-precision%29)))