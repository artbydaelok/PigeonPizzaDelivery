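; BP_DeliverySystem is an actor that picks the target locations for a delivery quest.
; On BeginPlay it sets the remaining delivery count and gathers every BP_DeliveryLocation in the level.
; It adds random unique picks until the requested count is reached, a loop that cannot finish if too few locations exist.
; The final loop over the chosen targets is still empty.
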(event EventBeginPlay
  (Variables|Default|SetDeliveriesRemaining (Variables|Default|GetNumberOfDeliveries))
  (bind _outactors (Actor|GetAllActorsOfClass "/Game/DeliveryQuestsSystem/BP_DeliveryLocation.BP_DeliveryLocation_C"))
  (Variables|Default|SetPossibleDeliveryLocations _outactors)
  (while (not (== (Utilities|Array|Length (Variables|Default|GetTargetDeliveryIndexes)) (Variables|Default|GetNumberOfDeliveries)))
    (Utilities|Array|AddUnique (Variables|Default|GetTargetDeliveryIndexes) (.OutItem (Utilities|Array|Random (Variables|Default|GetPossibleDeliveryLocations)))))
  (for _array_element (Variables|Default|GetTargetDeliveryIndexes)
    _))

(event Collision|EventActorBeginOverlap
  (params (OtherActor :type Actor%20Object%20Reference)))

(event EventTick
  (params (DeltaSeconds :type Float%20%28single-precision%29)))

(fn ConstructionScript)