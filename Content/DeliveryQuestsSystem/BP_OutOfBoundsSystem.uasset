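; Out-of-bounds manager that gives the player a short grace period to leave forbidden zones before losing.
; On BeginPlay it finds the third-person character and binds begin and end overlap events on every zone in OutOfBoundsZones.
; Entering a zone starts the lose timer; exiting cancels it only if the player overlaps no other zone.
; The lose state currently only prints a debug message.
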(event Custom|PlayerOutOfBounds
  (params (OverlappedActor :type Actor%20Object%20Reference) (OtherActor :type Actor%20Object%20Reference))
  ;[1 1 1] Binds all the Out Of Bound Zones to the event that will make the player lose if they are still outside.
  (if (== OtherActor (Variables|Default|GetPlayer))
    (bind _returnvalue (Utilities|Time|SetTimerbyEvent (delegate Custom|OutOfBoundsLoseState) 3.0))
    (Variables|Default|SetOutOfBoundsTimer _returnvalue)
    (Development|PrintString "Out Of Bounds")))

(event Custom|OutOfBoundsLoseState
  (Development|PrintString "Player loses due to being out of bounds."))

(event Custom|PlayerInBounds
  (params (OverlappedActor :type Actor%20Object%20Reference) (OtherActor :type Actor%20Object%20Reference))
  (if (== OtherActor (Variables|Default|GetPlayer))
    (bind _array_element (Utilities|Array|ForEachLoopwithBreak (Variables|Default|GetOutOfBoundsZones) :!label _label)
      (:LoopBody
        (if (Collision|IsOverlappingActor _array_element (Variables|Default|GetPlayer) :!class /Script/Engine.Actor)
          (Variables|Default|SetStillOutOfBounds true)
          (goto _label Break)))
      (:Completed
        (if (Variables|Default|GetStillOutOfBounds)
          (Development|PrintString "Player Still Out Of Bounds")
          (Variables|Default|SetStillOutOfBounds false)
          (else
            (Utilities|Time|ClearandInvalidateTimerbyHandle (Variables|Default|GetOutOfBoundsTimer))
            (Development|PrintString "Player In Bounds")
            (Variables|Default|SetStillOutOfBounds false)))))))

(event EventBeginPlay
  (bind _returnvalue (Actor|GetActorOfClass "/Game/ThirdPerson/Blueprints/BP_ThirdPersonCharacter.BP_ThirdPersonCharacter_C"))
  (Variables|Default|SetPlayer _returnvalue)
  ;[1 1 1] Binds all the Out Of Bound Zones to the event that will make the player lose if they are still outside.
  (for _array_element (Variables|Default|GetOutOfBoundsZones)
    (Collision|BindEventtoOnActorBeginOverlap _array_element (delegate Custom|PlayerOutOfBounds))
    (Collision|BindEventtoOnActorEndOverlap _array_element (delegate Custom|PlayerInBounds))))

(event Collision|EventActorBeginOverlap
  (params (OtherActor :type Actor%20Object%20Reference)))

(event EventTick
  (params (DeltaSeconds :type Float%20%28single-precision%29)))

(fn ConstructionScript)