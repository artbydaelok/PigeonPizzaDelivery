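; BP_DeliveryLocation is a pizza drop-off marker in the delivery quest system.
; On BeginPlay it caches the BP_DeliverySystem actor and plays a timeline that lerps the Arrow's relative Z between its start height and an AnimationAmount offset.
; When the player character overlaps PlayerDetect, it calls DeliverPizza on the delivery system and destroys itself.
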(event OnComponentBeginOverlap(PlayerDetect)
  (params (OverlappedComponent :type Primitive%20Component%20Object%20Reference) (OtherActor :type Actor%20Object%20Reference) (OtherComp :type Primitive%20Component%20Object%20Reference) (OtherBodyIndex :type Integer) (bFromSweep :type Boolean) (SweepResult :type Hit%20Result%20Structure%20%28by%20ref%29))
  (if (== OtherActor (Game|GetPlayerCharacter 0))
    (Default|DeliverPizza (Variables|Default|GetDeliverySystem))
    (Actor|DestroyActor)))

(event EventBeginPlay
  (bind _arrow (Variables|Default|GetArrow))
  (bind _returnvalue (Actor|GetActorOfClass "/Game/DeliveryQuestsSystem/BP_DeliverySystem.BP_DeliverySystem_C"))
  (Variables|Default|SetDeliverySystem _returnvalue)
  ;[1 1 1] Arrow Animation
  (Variables|Default|SetStart%20Relative%20Location (Variables|/Script/Engine.SceneComponent|GetRelativeLocation _arrow))
  (bind _alpha (Timeline|MoveArrowUpAndDown PlayFromStart)
    (:Update
      (Transformation|SetRelativeLocation _arrow (Math|Vector|MakeVector (.x (Variables|Default|GetStart%20Relative%20Location)) (.y (Variables|Default|GetStart%20Relative%20Location)) (Math|Float|Lerp (.z (Variables|Default|GetStart%20Relative%20Location)) (+ (.z (Variables|Default|GetStart%20Relative%20Location)) (Variables|Default|GetAnimationAmount)) _alpha)) false false))))

(event Collision|EventActorBeginOverlap
  (params (OtherActor :type Actor%20Object%20Reference)))

(event EventTick
  (params (DeltaSeconds :type Float%20%28single-precision%29)))

(fn ConstructionScript)